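; Base player character with single-axis movement, mode-based shooting, a ground-pound and a bounce for players landing on its top trigger.
; Attack modes select projectile class and cooldown, with Burst also spending recharging charges; shots take damage from PlayerStats.
; Jumping down boosts gravity and enables a collider that damages overlapped actors and spawns explosions.
; Crossing life-ratio steps when damaged adds or removes PlayerStats rewards, created by ModifiersGenerator; death only prints.
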(event `Teleported_Event`
  (`KismetSystemLibrary.Delay` 0.2)
  (set `self.JustTeleported` false))

(event `self.ReceiveBeginPlay`
  (bind _charactermovement (`self.CharacterMovement`))
  (set `self.BaseGravityScale` (`CharacterMovementComponent.GravityScale` _charactermovement))
  (set `self.BaseAirControl` (`CharacterMovementComponent.AirControl` _charactermovement))
  (set `PrimitiveComponent.bGenerateOverlapEvents` false (`self.JumpDownCollider`)))

(event `Key|U`
  (params (Key :type "Key Structure" :default "AnyKey"))
  (:`Pressed`
    (`KismetSystemLibrary.PrintString` "NORMAL")
    (`self.SetAttackMode` "NewEnumerator0")
    (`self.ResetAttackCooldown` :!label _label)))

(event `Key|I`
  (params (Key :type "Key Structure" :default "AnyKey"))
  (:`Pressed`
    (`KismetSystemLibrary.PrintString` "BURST")
    (`self.SetAttackMode` "NewEnumerator1")
    (goto _label)))

(event `self.ReceiveAnyDamage`
  (params (Damage :type "Float (single-precision)") (DamageType :type "DamageType Object Reference") (InstigatedBy :type "Controller Object Reference") (DamageCauser :type "Actor Object Reference"))
  (`self.ReceiveDamage` Damage))

(event `self.JumpDownCollider.OnComponentBeginOverlap`
  (params (OverlappedComponent :type "PrimitiveComponent Object Reference") (OtherActor :type "Actor Object Reference") (OtherComp :type "PrimitiveComponent Object Reference") (OtherBodyIndex :type Integer) (bFromSweep :type Boolean) (SweepResult :type "HitResult Structure (by ref)"))
  (if (!= OtherActor self)
    (`GameplayStatics.ApplyDamage` OtherActor 10.0)
    (`|SpawnActorFromClass` "/Game/StarterContent/Blueprints/Blueprint_Effect_Explosion.Blueprint_Effect_Explosion_C" (`self.GetTransform`) "Undefined" "OverrideRootScale")))

(event `self.TopTrigger.OnComponentBeginOverlap`
  (params (OverlappedComponent :type "PrimitiveComponent Object Reference") (OtherActor :type "Actor Object Reference") (OtherComp :type "PrimitiveComponent Object Reference") (OtherBodyIndex :type Integer) (bFromSweep :type Boolean) (SweepResult :type "HitResult Structure (by ref)"))
  (if (!= OtherActor self)
    (bind _asplayer_base (cast `/Game/Blueprints/PlayerBase` OtherActor))
    (`self.MyJump` _asplayer_base)))

(fn `JumpDown`
  (bind _charactermovement (`self.CharacterMovement`))
  (if (`NavMovementComponent.IsFalling` _charactermovement)
    (`MovementComponent.StopMovementImmediately` _charactermovement)
    (set `CharacterMovementComponent.AirControl` 0.0 _charactermovement)
    (set `CharacterMovementComponent.GravityScale` (* (`CharacterMovementComponent.GravityScale` _charactermovement) (`self.GravityScaleModifier`)) _charactermovement)
    (set `PrimitiveComponent.bGenerateOverlapEvents` true (`self.JumpDownCollider`))
    (set `self.JumpingDown` true)))

(fn `Move`
  (params (AxisValue :type "Float (double-precision)"))
  (locals (TempRot :type "Rotator Structure"))
  (`self.AddMovementInput` (0.0 -1.0 0.0) AxisValue)
  (if (> AxisValue 0.0)
    (set `local.TempRot` (struct :`Yaw` -90.0))
    (`self.K2_SetActorRotation` (`local.TempRot`) :!label _label)
    (elif (< AxisValue 0.0)
      (set `local.TempRot` (struct :`Yaw` 90.0))
      (goto _label))))

(fn `MyJump`
  (`self.Jump`))

(fn `MyStopJumping`
  (`self.StopJumping`))

(fn `ReceiveDamage`
  (params (damage :type "Float (double-precision)"))
  (locals (tempHPRatioBefore :type Integer) (tempHPRatioAfter :type Integer))
  (bind _playerstats (`self.PlayerStats`))
  (bind _temphpratiobefore (`local.tempHPRatioBefore`))
  (bind _temphpratioafter (`local.tempHPRatioAfter`))
  (bind _returnvalue (!= (`KismetMathLibrary.Abs_Int` (- _temphpratiobefore _temphpratioafter)) 0))
  (bind _result (`/Game/Blueprints/PlayerStats.GetCurrentLifeRatio` _playerstats))
  (set `local.tempHPRatioBefore` (`KismetMathLibrary.FTrunc` (/ _result 10.0)))
  (bind _output_get (set `/Game/Blueprints/PlayerStats.hp` (- (`/Game/Blueprints/PlayerStats.hp` _playerstats) (`KismetMathLibrary.FTrunc` damage)) _playerstats))
  (bind _result_2 (`/Game/Blueprints/PlayerStats.GetCurrentLifeRatio` _playerstats))
  (set `local.tempHPRatioAfter` (`KismetMathLibrary.FTrunc` (/ _result_2 10.0)))
  (if (<= _output_get 0)
    (`KismetSystemLibrary.PrintString` "Dead")
    (else
      ;[1 1 1] > ha perdido vida; < ha ganado vida
      (`/Engine/EditorBlueprintResources/StandardMacros.CompareInt` _temphpratiobefore _temphpratioafter
        (:`>`
          (while _returnvalue
            (bind _type (`/Game/Blueprints/ModifiersGenerator.CreateModifier` (`self.ModifiersGenerator`)))
            (`/Game/Blueprints/PlayerStats.AddReward` _playerstats _type)
            (`/Engine/EditorBlueprintResources/StandardMacros.IncrementInt` _temphpratioafter)))
        (:`<`
          (while _returnvalue
            (`/Game/Blueprints/PlayerStats.RemoveReward` (`self.PlayerStats`))
            (`/Engine/EditorBlueprintResources/StandardMacros.IncrementInt` _temphpratioafter)))))))

(fn `ResetAttackCooldown`
  (set `self.ShootTimer` 1e+44))

(fn `ResetJumpDown`
  (bind _charactermovement (`self.CharacterMovement`))
  (set `CharacterMovementComponent.GravityScale` (`self.BaseGravityScale`) _charactermovement)
  (set `CharacterMovementComponent.AirControl` (`self.BaseAirControl`) _charactermovement)
  (set `PrimitiveComponent.bGenerateOverlapEvents` false (`self.JumpDownCollider`)))

(fn `ResetJumpDownIfOnTheGround`
  (if (`self.JumpingDown`)
    (if (not (`NavMovementComponent.IsFalling` (`self.CharacterMovement`)))
      (`self.ResetJumpDown`))))

(fn `SetAttackMode`
  (params (NewAttackMode :type "/Game/Blueprints/Attack_Mode Enum"))
  (bind _output_get (set `self.AttackMode` NewAttackMode))
  (switch `/Game/Blueprints/Attack_Mode` _output_get
    (:`NewEnumerator0`
      (set `self.ShootCooldown` (`self.ShootNormalCooldown`))
      (set `self.CurrentProjectileClass` "/Game/Blueprints/Projectiles/PlayerProjectileNormal.PlayerProjectileNormal_C"))
    (:`NewEnumerator1`
      (set `self.ShootCooldown` (`self.ShootBurstCooldown`))
      (set `self.CurrentProjectileClass` "/Game/Blueprints/Projectiles/PlayerProjectileBurst.PlayerProjectileBurst_C"))
    (:`NewEnumerator2`
      (set `self.ShootCooldown` (`self.ShootBurstCooldown`))
      (set `self.CurrentProjectileClass` "/Game/Blueprints/Projectiles/PlayerProjectileBounce.PlayerProjectileBounce_C"))
    (:`NewEnumerator3`
      (set `self.ShootCooldown` (`self.ShootBurstCooldown`))
      (set `self.CurrentProjectileClass` "/Game/Blueprints/Projectiles/PlayerProjectileTriple.PlayerProjectileTriple_C"))
    (:`NewEnumerator4`
      (set `self.ShootCooldown` (`self.ShootBurstCooldown`))
      (set `self.CurrentProjectileClass` "/Game/Blueprints/Projectiles/PlayerProjectileBig.PlayerProjectileBig_C"))))

(fn `Shoot`
  (if (>= (`self.ShootTimer`) (`self.ShootCooldown`))
    (set `self.ShootTimer` 0.0)
    (switch `/Game/Blueprints/Attack_Mode` (`self.AttackMode`)
      (:`NewEnumerator0`
        (`self.ShootProjectile` :!label _label))
      (:`NewEnumerator1`
        (if (> (`self.BurstCharges`) 0)
          (`self.ShootProjectile`)
          (`/Engine/EditorBlueprintResources/StandardMacros.DecrementInt` (`self.BurstCharges`))))
      (:`NewEnumerator2`
        (goto _label))
      (:`NewEnumerator3`
        (goto _label))
      (:`NewEnumerator4`
        (goto _label)))))

(fn `ShootProjectile`
  (bind _asplayer_projectile_base (castclass `/Game/Blueprints/Projectiles/PlayerProjectileBase` (`self.CurrentProjectileClass`)))
  (bind _currentdamage (`/Game/Blueprints/PlayerStats.GetCurrentDamage` (`self.PlayerStats`)))
  (`|SpawnActorFromClass` _asplayer_projectile_base (`SceneComponent.K2_GetComponentToWorld` (`self.SpawnProjectilePoint`)) "Undefined" "OverrideRootScale" null _currentdamage))

(fn `UpdateBurstCharges`
  (params (DeltaTime :type "Float (double-precision)"))
  (if (< (`self.BurstCharges`) (`self.MaxBurstCharges`))
    (if (>= (`self.BurstChargeTimer`) (`self.BurstChargeCooldown`))
      (`/Engine/EditorBlueprintResources/StandardMacros.IncrementInt` (`self.BurstCharges`)
        (:`  `
          (set `self.BurstChargeTimer` 0.0)))
      (else
        (set `self.BurstChargeTimer` (+ (`self.BurstChargeTimer`) DeltaTime))))
    (else
      (set `self.BurstChargeTimer` 0.0))))

(fn `UpdateShootTimer`
  (params (DeltaTime :type "Float (double-precision)"))
  (set `self.ShootTimer` (+ DeltaTime (`self.ShootTimer`))))

(fn `UserConstructionScript`)