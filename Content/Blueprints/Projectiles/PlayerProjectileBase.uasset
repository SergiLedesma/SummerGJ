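; Base player projectile actor that damages what it overlaps and explodes on impact or after a short lifetime.
; Overlaps ignore the instigator and actors of its own class, and a DoOnce lets only the first valid hit apply damage.
; Both hit and timeout spawn an explosion effect, play a 2D explosion sound and destroy the actor, though timeout calls destroy before spawning the effect.
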(event `self.ReceiveBeginPlay`
  (`KismetSystemLibrary.Delay` 3.0)
  (`self.K2_DestroyActor`)
  (`|SpawnActorFromClass` "/Game/StarterContent/Blueprints/Blueprint_Effect_Explosion.Blueprint_Effect_Explosion_C" (`self.GetTransform`) "Undefined" "OverrideRootScale")
  (`GameplayStatics.PlaySound2D` "/Game/SoundFX/ExplosionCue.ExplosionCue" 0.8))

(event `self.ReceiveActorBeginOverlap`
  (params (OtherActor :type "Actor Object Reference"))
  (if (!= OtherActor (`self.GetInstigator`))
    (if (!= (`GameplayStatics.GetObjectClass` OtherActor) (`GameplayStatics.GetObjectClass` self))
      (`/Engine/EditorBlueprintResources/StandardMacros.DoOnce` false
        (:`Completed`
          (`GameplayStatics.ApplyDamage` OtherActor (`self.damage`))
          (`|SpawnActorFromClass` "/Game/StarterContent/Blueprints/Blueprint_Effect_Explosion.Blueprint_Effect_Explosion_C" (`self.GetTransform`) "Undefined" "OverrideRootScale")
          (`GameplayStatics.PlaySound2D` "/Game/SoundFX/ExplosionCue.ExplosionCue" 0.8)
          (`self.K2_DestroyActor`))))))

(fn `UserConstructionScript`)