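; ModifiersGenerator hands out random modifiers from a limited pool, with three copies of each of three enum types seeded on BeginPlay.
; CreateModifier picks from ModifiersList using a random index bounded by the Modifiers map size, then decrements that type's remaining count in the map.
; At zero it removes the map key, but the list removal rolls a new random index, so it can drop a different entry than the exhausted one.
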(event `self.ReceiveBeginPlay`
  (bind _modifiers (`self.modifiers`))
  (`BlueprintMapLibrary.Map_Add` _modifiers "NewEnumerator0" 3)
  (`BlueprintMapLibrary.Map_Add` _modifiers "NewEnumerator1" 3)
  (`BlueprintMapLibrary.Map_Add` _modifiers "NewEnumerator2" 3))

(fn `CreateModifier`
  (returns (type :type "/Game/Blueprints/Modifier_types Enum"))
  (locals (GeneratedNumber :type Integer) (result :type "/Game/Blueprints/Modifier_types Enum"))
  (bind _modifiers (`self.modifiers`))
  (bind _result (`local.result`))
  (bind _returnvalue (`KismetMathLibrary.RandomIntegerInRange` 0 (- (`BlueprintMapLibrary.Map_Length` _modifiers) 1)))
  (bind _output_get (set `local.result` (`|GetArrayItem` (`self.modifiersList`) _returnvalue)))
  (bind _returnvalue_2 (- (`BlueprintMapLibrary.Map_Find` _modifiers _output_get) 1))
  (if (== _returnvalue_2 0)
    (`BlueprintMapLibrary.Map_Remove` _modifiers _result)
    (`KismetArrayLibrary.Array_Remove` (`self.modifiersList`) _returnvalue)
    (else
      (`BlueprintMapLibrary.Map_Add` _modifiers _result _returnvalue_2)))
  (return _result))