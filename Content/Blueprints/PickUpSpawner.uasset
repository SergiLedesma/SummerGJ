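; PickUp spawner that periodically spawns a PickUps actor at a random free PickUpSpawnPoint in the level.
; BeginPlay caches spawn point transforms and marks every index free in a map, with a looping retriggerable delay driving spawns every two seconds.
; Each spawn removes its index from the free map and passes it to the pickup.
; RemoveSpawnPointUsage returns an index to the free pool.
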(event `self.ReceiveBeginPlay`
  ;[1 1 1] Init Spawpoints List
  (bind _outactors (`GameplayStatics.GetAllActorsOfClass` "/Game/Blueprints/PickUpSpawnPoint.PickUpSpawnPoint_C"))
  (for (_array_element _array_index) _outactors
    (`KismetArrayLibrary.Array_Add` (`self.SpawnPoints`) (`self.GetTransform` _array_element))
    (`BlueprintMapLibrary.Map_Add` (`self.SpawnPointsFree`) _array_index _array_index)
    (`KismetSystemLibrary.RetriggerableDelay` 2.0 :!label _label)
    (`self.SpawnAtRandomSpawnPoint`)
    (goto _label)))

(fn `RemoveSpawnPointUsage`
  (params (Index :type Integer))
  (`BlueprintMapLibrary.Map_Add` (`self.SpawnPointsFree`) Index Index))

(fn `SpawnAtRandomSpawnPoint`
  (if (!= (`BlueprintMapLibrary.Map_Length` (`self.SpawnPointsFree`)) 0)
    (bind _output_get (set `self.AuxRand` (`KismetMathLibrary.RandomIntegerInRange` 0 (- (`BlueprintMapLibrary.Map_Length` (`self.SpawnPointsFree`)) 1))))
    (bind _keys (`BlueprintMapLibrary.Map_Keys` (`self.SpawnPointsFree`)))
    (bind _output (`|GetArrayItem` _keys _output_get))
    (set `self.RandomGenerated` _output)
    (`BlueprintMapLibrary.Map_Remove` (`self.SpawnPointsFree`) _output)
    (`|SpawnActorFromClass` "/Game/Blueprints/PickUps.PickUps_C" (`|GetArrayItem` (`self.SpawnPoints`) (`self.RandomGenerated`)) "Undefined" "OverrideRootScale" null (`self.RandomGenerated`))))

(fn `UserConstructionScript`)