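; Player projectile that damages what it hits and explodes.
; Half a second after BeginPlay, Tick starts pushing BulletCollision forward every frame with an impulse scaled from the ProjectileMovement initial speed plus delta time.
; The first overlap with an actor other than its instigator or another projectile of the same class applies damage, spawns an explosion effect and destroys the projectile.
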(event `self.ReceiveTick`
  (params (DeltaSeconds :type "Float (single-precision)"))
  (bind _bulletcollision (`self.BulletCollision`))
  (if (`self.enabletick`)
    (`PrimitiveComponent.AddImpulse` _bulletcollision (* (`SceneComponent.GetForwardVector` _bulletcollision) (* (+ DeltaSeconds (`ProjectileMovementComponent.InitialSpeed` (`self.ProjectileMovement`))) 5.0)) "None" false)))

(event `self.ReceiveBeginPlay`
  (`KismetSystemLibrary.Delay` 0.5)
  (set `self.enabletick` true))

(event `self.ReceiveActorBeginOverlap`
  (params (OtherActor :type "Actor Object Reference"))
  (if (!= OtherActor (`self.GetInstigator`))
    (if (!= (`GameplayStatics.GetObjectClass` OtherActor) (`GameplayStatics.GetObjectClass` self))
      (`/Engine/EditorBlueprintResources/StandardMacros.DoOnce` false
        (:`Completed`
          (`GameplayStatics.ApplyDamage` OtherActor 10.0)
          (`|SpawnActorFromClass` "/Game/StarterContent/Blueprints/Blueprint_Effect_Explosion.Blueprint_Effect_Explosion_C" (`self.GetTransform`) "Undefined" "OverrideRootScale")
          (`self.K2_DestroyActor`))))))

(fn `UserConstructionScript`)