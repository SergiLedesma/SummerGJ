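; Pickup actor that grants one of the two players a special attack mode.
; The construction script rolls one of four non-Normal types at random and sets the matching mesh and material.
; On overlap with player character 0 or 1, it applies that type and resets the player's attack cooldown.
; It then frees its spawn point index on the first PickUpSpawner found in the level and destroys itself.
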(event `self.ReceiveActorBeginOverlap`
  (params (OtherActor :type "Actor Object Reference"))
  (bind _returnvalue (`GameplayStatics.GetPlayerCharacter` 1))
  (bind _returnvalue_2 (`GameplayStatics.GetPlayerCharacter` 0))
  (if (== OtherActor _returnvalue_2)
    (bind _asplayer_base (cast `/Game/Blueprints/PlayerBase` _returnvalue_2))
    (set `self.OtherPlayer` _asplayer_base)
    (`/Game/Blueprints/PlayerBase.SetAttackMode` (`self.OtherPlayer`) (`self.Type`) :!label _label)
    (`/Game/Blueprints/PlayerBase.ResetAttackCooldown` (`self.OtherPlayer`))
    (bind _outactors (`GameplayStatics.GetAllActorsOfClass` "/Game/Blueprints/PickUpSpawner.PickUpSpawner_C"))
    (`/Game/Blueprints/PickUpSpawner.RemoveSpawnPointUsage` (`|GetArrayItem` _outactors) (`self.SpawnPointIndex`))
    (`self.K2_DestroyActor`)
    (elif (== OtherActor _returnvalue)
      (bind _asplayer_base_2 (cast `/Game/Blueprints/PlayerBase` _returnvalue))
      (set `self.OtherPlayer` _asplayer_base_2)
      (goto _label))))

(fn `UserConstructionScript`
  (bind _mesh (`self.Mesh`))
  (bind _mesh_2 (`self.Mesh`))
  (bind _output_get (set `self.Type` (select `int` (`KismetMathLibrary.RandomInteger` 4) :`0` "NewEnumerator4" :`1` "NewEnumerator1" :`2` "NewEnumerator2" :`3` "NewEnumerator3" :!type "/Game/Blueprints/Attack_Mode Enum")))
  (switch `/Game/Blueprints/Attack_Mode` _output_get
    (:`NewEnumerator0`
      (`StaticMeshComponent.SetStaticMesh` _mesh "/Game/Models/PickupBasic.PickupBasic")
      (`PrimitiveComponent.SetMaterial` _mesh_2 0 "/Game/Models/PickupBasic1.PickupBasic1"))
    (:`NewEnumerator1`
      (`StaticMeshComponent.SetStaticMesh` _mesh "/Game/Models/PickupBurst.PickupBurst")
      (`PrimitiveComponent.SetMaterial` _mesh_2 0 "/Game/Models/PickupBurst1.PickupBurst1"))
    (:`NewEnumerator2`
      (`StaticMeshComponent.SetStaticMesh` _mesh "/Game/Models/PickupBouncing.PickupBouncing")
      (`PrimitiveComponent.SetMaterial` _mesh_2 0 "/Game/Models/PickupBouncing1.PickupBouncing1"))
    (:`NewEnumerator3`
      (`StaticMeshComponent.SetStaticMesh` _mesh "/Game/Models/PickupTriple.PickupTriple")
      (`PrimitiveComponent.SetMaterial` _mesh_2 0 "/Game/Models/PickupTriple1.PickupTriple1"))
    (:`NewEnumerator4`
      (`StaticMeshComponent.SetStaticMesh` _mesh "/Game/Models/PickupBig.PickupBig")
      (`PrimitiveComponent.SetMaterial` _mesh_2 0 "/Game/Models/PickupBig1.PickupBig1"))))