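; Base player projectile Actor that damages what it overlaps, explodes and destroys itself, or expires after a fixed lifetime.
; Overlaps with the instigator or with projectiles of the same class are ignored.
; The first valid overlap passes a DoOnce, applies Damage, prints the returned amount and spawns an explosion effect.
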(event `self.ReceiveBeginPlay`
  (`KismetSystemLibrary.Delay` 5.0)
  (`self.K2_DestroyActor`))

(event `self.ReceiveActorBeginOverlap`
  (params (OtherActor :type "Actor Object Reference"))
  (if (!= OtherActor (`self.GetInstigator`))
    (if (!= (`GameplayStatics.GetObjectClass` OtherActor) (`GameplayStatics.GetObjectClass` self))
      (`/Engine/EditorBlueprintResources/StandardMacros.DoOnce` false
        (:`Completed`
          (bind _returnvalue (`GameplayStatics.ApplyDamage` OtherActor (`self.damage`)))
          (`KismetSystemLibrary.PrintText` (`KismetTextLibrary.Conv_DoubleToText` _returnvalue "HalfToEven"))
          (`|SpawnActorFromClass` "/Game/StarterContent/Blueprints/Blueprint_Effect_Explosion.Blueprint_Effect_Explosion_C" (`self.GetTransform`) "Undefined" "OverrideRootScale")
          (`self.K2_DestroyActor`))))))

(fn `UserConstructionScript`)