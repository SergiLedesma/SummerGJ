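; Player0 is a child player Blueprint that binds the 0-suffixed input mappings for movement, shooting and jumping to Move, Shoot, MyJump and MyStopJumping, none of which are defined here.
; Holding Jump0 opens a Gate that re-enters itself through a short retriggerable delay, calling MyJump repeatedly.
; Releasing Jump0 calls MyStopJumping and closes the Gate.
; The construction script only calls its parent.
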(event `InputAxis|MoveRight0`
  (params (AxisValue :type "Float (single-precision)"))
  (`self.Move` AxisValue))

(event `InputAction|Shoot0`
  (params (Key :type "Key Structure" :default "AnyKey"))
  (:`Pressed`
    (`self.Shoot`)))

(event `InputAction|Jump0`
  (params (Key :type "Key Structure" :default "AnyKey"))
  (:`Pressed`
    (`|ExecutionSequence`
      (:`then_0`
        (goto _label :!via `Open`))
      (:`then_1`
        (`/Engine/EditorBlueprintResources/StandardMacros.Gate` true :!label _label
          (:`Exit`
            (`self.MyJump`)
            (`KismetSystemLibrary.RetriggerableDelay` 0.02)
            (goto _label))))))
  (:`Released`
    (`self.MyStopJumping`)
    (goto _label :!via `Close`)))

(fn `UserConstructionScript`
  (`parent.UserConstructionScript`))