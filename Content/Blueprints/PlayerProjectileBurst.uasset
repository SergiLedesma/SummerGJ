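; Player burst projectile that gets a forward push shortly after spawning and destroys itself after five seconds.
; BeginPlay enables the push after a short delay, then Tick applies an impulse along BulletCollision's forward vector every frame.
; The impulse scales ProjectileMovement's InitialSpeed by ProjectileMultiplier, with DeltaSeconds added rather than multiplied, so total push depends on frame rate.
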(event `self.ReceiveTick`
  (params (DeltaSeconds :type "Float (single-precision)"))
  (bind _bulletcollision (`self.BulletCollision`))
  (if (`self.enabletick`)
    (`PrimitiveComponent.AddImpulse` _bulletcollision (* (`SceneComponent.GetForwardVector` _bulletcollision) (* (+ DeltaSeconds (`ProjectileMovementComponent.InitialSpeed` (`self.ProjectileMovement`))) (`self.ProjectileMultiplier`))) "None" false)))

(event `self.ReceiveBeginPlay`
  (`KismetSystemLibrary.Delay` 0.5)
  (set `self.enabletick` true)
  (`KismetSystemLibrary.Delay` 4.5)
  (`self.K2_DestroyActor`))

(fn `UserConstructionScript`)